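; BP_Button is a toggle button actor that publishes its on/off state to a CLIPS client as a condition fact.
; Each overlap with its Box flips IsOn, then ChangeMat swaps the mesh material and asserts or retracts the fact keyed by ButtonID.
; BeginPlay runs the same update, so the material and fact match the initial state.
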(event OnComponentBeginOverlap(Box)
  (params (OtherActor :type Actor%20Object%20Reference) (OtherComp :type Primitive%20Component%20Object%20Reference) (OtherBodyIndex :type Integer) (bFromSweep :type Boolean) (SweepResult :type Hit%20Result%20Structure%20%28by%20ref%29))
  (if (Variables|Default|GetIsOn)
    (Variables|Default|SetIsOn false)
    (else
      (Variables|Default|SetIsOn true)))
  (CallFunction|ChangeMat))

(event Custom|ChangeMat
  (bind _button_id (Variables|Default|GetButton_ID))
  (bind _clipsclient (Variables|Default|GetCLIPSClient))
  (bind _staticmesh (Variables|Default|GetStaticMesh))
  (if (Variables|Default|GetIsOn)
    (Rendering|Material|SetMaterial _staticmesh 1 (Variables|Default|GetM_On))
    (Class|CLIPSClient|AssertFact _clipsclient "condicion" _button_id)
    (else
      (Rendering|Material|SetMaterial _staticmesh 1 (Variables|Default|GetM_Off))
      (Class|CLIPSClient|RetractFact _clipsclient "condicion" _button_id))))

(event EventBeginPlay
  (CallFunction|ChangeMat))

(event EventTick
  (params (DeltaSeconds :type Float%20%28single-precision%29)))

(fn ConstructionScript)