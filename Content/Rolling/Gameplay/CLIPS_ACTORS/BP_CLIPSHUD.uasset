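; BP_CLIPSHUD is an actor that puts an on-screen readout of CLIPS rule-engine facts on the viewport through a W_Facts widget.
; On a timed Tick refresh, it clears the game mode's CLIPS output and queries all condicion and evento facts, printing their indices and ids to an "unreal" router.
; Query results copy that output into Facts on this actor, which the widget references as its HUD.
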(event OnQueryResult(CLIPSClient)
  (params (Result :type String))
  (bind _returnvalue (Class|CLIPSComponent|CLIPSOutput (Variables|/Game/Rolling/Gameplay/CLIPS_ACTORS/CLIPS_GM.CLIPS_GM_C|GetCLIPS (Variables|Default|GetGM))))
  (Variables|Default|SetFacts _returnvalue))

(event EventBeginPlay
  (bind _asclips_gm (Utilities|Casting|CastToCLIPS_GM (Game|GetGameMode)))
  (Variables|Default|SetGM _asclips_gm)
  (bind _returnvalue (UserInterface|CreateWidget "/Game/Rolling/Gameplay/CLIPS_ACTORS/W_Facts.W_Facts_C" (Game|GetPlayerController 0)))
  (bind _output_get (Variables|Default|SetW_Facts _returnvalue))
  (Variables|/Game/Rolling/Gameplay/CLIPS_ACTORS/W_Facts.W_Facts_C|SetHUD _output_get self)
  (UserInterface|Viewport|AddtoViewport _output_get 0))

(event Collision|EventActorBeginOverlap
  (params (OtherActor :type Actor%20Object%20Reference)))

(event EventTick
  (params (DeltaSeconds :type Float%20%28single-precision%29))
  (bind _clipsclient (Variables|Default|GetCLIPSClient))
  (bind _output_get (Variables|Default|SetTimeSinceRefresh (+ DeltaSeconds (Variables|Default|GetTimeSinceRefresh))))
  (if (>= _output_get (Variables|Default|GetRefreshTime))
    (Variables|Default|SetTimeSinceRefresh 0.0)
    (Class|CLIPSComponent|CLIPSClear (Variables|/Game/Rolling/Gameplay/CLIPS_ACTORS/CLIPS_GM.CLIPS_GM_C|GetCLIPS (Variables|Default|GetGM)))
    (Class|CLIPSClient|EvalQuery _clipsclient "(do-for-all-facts ((?c condicion)) TRUE (printout unreal \"<Fact-\" (fact-index ?c) \"> -> \" ?c:id crlf))")
    (Class|CLIPSClient|EvalQuery _clipsclient "(do-for-all-facts ((?c evento)) TRUE (printout unreal \"<Fact-\" (fact-index ?c) \"> -> \" ?c:id crlf))")))

(fn ConstructionScript)