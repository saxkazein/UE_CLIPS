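; BP_Event-NOCLIPS is an actor whose Cube shows an on or off state through its material.
; On Tick, while Updated is false, it applies MATON or MATOFF to the Cube according to Active, then sets Updated.
; Updated acts as a latch that avoids repeat material swaps; nothing in these graphs clears it or changes Active.
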(event EventBeginPlay)

(event Collision|EventActorBeginOverlap
  (params (OtherActor :type Actor%20Object%20Reference)))

(event EventTick
  (params (DeltaSeconds :type Float%20%28single-precision%29))
  (bind _cube (Variables|Default|GetCube))
  (if (not (Variables|Default|GetUpdated))
    (if (Variables|Default|GetActive)
      (Rendering|Material|SetMaterial _cube 0 (Variables|Default|GetMAT_ON))
      (Variables|Default|SetUpdated true)
      (else
        (Rendering|Material|SetMaterial _cube 0 (Variables|Default|GetMAT_OFF))
        (Variables|Default|SetUpdated true)))))

(fn ConstructionScript)