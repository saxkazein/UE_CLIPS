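; BP_Ball is a player-controlled physics ball that rolls relative to the camera and resets on hazards.
; MoveForward and MoveRight apply horizontal impulse and scaled torque along the camera-to-ball direction and its perpendicular, while right-stick X yaws the spring arm.
; Overlapping an actor named "DeadTrigger" teleports it to its BeginPlay position and zeroes its velocities.
; Q and E set CamRot, but nothing here uses that value.
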(event EventBeginPlay
  (Variables|Default|SetInitialPos (Transformation|GetWorldLocation (Variables|Default|GetBall))))

(event Collision|EventActorBeginOverlap
  (params (OtherActor :type Actor%20Object%20Reference))
  (bind _ball (Variables|Default|GetBall))
  (if (Utilities|Enum|Equal(Enum) (Utilities|GetDisplayName OtherActor) "DeadTrigger")
    (Transformation|Teleport (Variables|Default|GetInitialPos) (Transformation|GetWorldRotation (Variables|Default|GetBall)))
    (Physics|SetPhysicsLinearVelocity _ball "0, 0, 0" false "None")
    (Class|PrimitiveComponent|SetPhysicsAngularVelocity _ball "0, 0, 0" false "None")))

(event EventTick
  (params (DeltaSeconds :type Float%20%28single-precision%29)))

(event Input|AxisEvents|InputAxisMoveRight
  (params (AxisValue :type Float%20%28single-precision%29))
  (bind _returnvalue (* AxisValue 1.0))
  (bind _ball (Variables|Default|GetBall))
  (bind _camera (Variables|Default|GetCamera))
  (bind _impulse (Variables|Default|GetImpulse))
  (bind _returnvalue_2 (Transformation|GetWorldLocation _camera))
  (bind _returnvalue_3 (Transformation|GetWorldLocation _ball))
  (bind _returnvalue_4 (* _returnvalue _impulse))
  (bind _returnvalue_5 (Class|KismetMathLibrary|GetDirectionVector _returnvalue_2 _returnvalue_3))
  (bind _returnvalue_6 (Math|Vector|RotateVector _returnvalue_5 "0,90.000000, 0"))
  (bind (_x _y) (Math|Vector|BreakVector _returnvalue_6))
  (bind _returnvalue_7 (* _returnvalue_4 _y))
  (bind _returnvalue_8 (* _x _returnvalue_4))
  (Physics|AddImpulse (Variables|Default|GetBall) (Math|Vector|MakeVector _returnvalue_8 _returnvalue_7 0.0) "None" false)
  (Class|PrimitiveComponent|AddTorque (Variables|Default|GetBall) (* (Math|Vector|MakeVector (* _returnvalue_7 -1.0) _returnvalue_8 0.0) (Variables|Default|GetMultiTorque)) "None" false))

(event Input|AxisEvents|InputAxisMoveForward
  (params (AxisValue :type Float%20%28single-precision%29))
  (bind _ball (Variables|Default|GetBall))
  (bind _camera (Variables|Default|GetCamera))
  (bind _impulse (Variables|Default|GetImpulse))
  (bind _returnvalue (Transformation|GetWorldLocation _camera))
  (bind _returnvalue_2 (Transformation|GetWorldLocation _ball))
  (bind _returnvalue_3 (* AxisValue _impulse))
  (bind _returnvalue_4 (Class|KismetMathLibrary|GetDirectionVector _returnvalue _returnvalue_2))
  (bind (_x _y) (Math|Vector|BreakVector _returnvalue_4))
  (bind _returnvalue_5 (* _returnvalue_3 _y))
  (bind _returnvalue_6 (* _x _returnvalue_3))
  (Physics|AddImpulse (Variables|Default|GetBall) (Math|Vector|MakeVector _returnvalue_6 _returnvalue_5 0.0) "None" false)
  (Class|PrimitiveComponent|AddTorque (Variables|Default|GetBall) (* (Math|Vector|MakeVector _returnvalue_5 _returnvalue_6 0.0) (Variables|Default|GetMultiTorque)) "None" false))

(event Input|GamepadEvents|GamepadRightX
  (params (AxisValue :type Float%20%28single-precision%29))
  (Transformation|AddRelativeRotation (Variables|Default|GetSpringArm) (Class|KismetMathLibrary|MakeRot 0.0 AxisValue 0.0) false))

(event Input|KeyboardEvents|Q
  (:Pressed
    (Variables|Default|SetCamRot 5.0))
  (:Released
    (Variables|Default|SetCamRot 0.0)))

(event Input|KeyboardEvents|E
  (:Pressed
    (Variables|Default|SetCamRot -5.0))
  (:Released
    (Variables|Default|SetCamRot 0.0)))

(fn ConstructionScript)