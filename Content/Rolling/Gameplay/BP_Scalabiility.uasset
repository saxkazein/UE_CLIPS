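; BP_Scalabiility is a debug-style actor that switches engine scalability presets at runtime through console commands.
; On BeginPlay it applies the lowest preset, cutting resolution scale and dropping all other quality groups to minimum.
; Releasing F1 reapplies that low preset, and releasing F2 sets full resolution with the top quality level for each group.
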(event EventBeginPlay
  (Development|ExecuteConsoleCommand "sg.ResolutionQuality 25")
  (Development|ExecuteConsoleCommand "sg.ViewDistanceQuality 0")
  (Development|ExecuteConsoleCommand "sg.AntiAliasingQuality 0")
  (Development|ExecuteConsoleCommand "sg.PostProcessQuality 0")
  (Development|ExecuteConsoleCommand "sg.ShadowQuality 0")
  (Development|ExecuteConsoleCommand "sg.TextureQuality 0")
  (Development|ExecuteConsoleCommand "sg.EffectsQuality 0"))

(event Collision|EventActorBeginOverlap
  (params (OtherActor :type Actor%20Object%20Reference)))

(event EventTick
  (params (DeltaSeconds :type Float%20%28single-precision%29)))

(event Input|KeyboardEvents|F1
  (:Released
    (Development|ExecuteConsoleCommand "sg.ResolutionQuality 25")
    (Development|ExecuteConsoleCommand "sg.ViewDistanceQuality 0")
    (Development|ExecuteConsoleCommand "sg.AntiAliasingQuality 0")
    (Development|ExecuteConsoleCommand "sg.PostProcessQuality 0")
    (Development|ExecuteConsoleCommand "sg.ShadowQuality 0")
    (Development|ExecuteConsoleCommand "sg.TextureQuality 0")
    (Development|ExecuteConsoleCommand "sg.EffectsQuality 0")))

(event Input|KeyboardEvents|F2
  (:Released
    (Development|ExecuteConsoleCommand "sg.ResolutionQuality 100")
    (Development|ExecuteConsoleCommand "sg.ViewDistanceQuality 4")
    (Development|ExecuteConsoleCommand "sg.AntiAliasingQuality 4")
    (Development|ExecuteConsoleCommand "sg.PostProcessQuality 4")
    (Development|ExecuteConsoleCommand "sg.ShadowQuality 4")
    (Development|ExecuteConsoleCommand "sg.TextureQuality 4")
    (Development|ExecuteConsoleCommand "sg.EffectsQuality 4")))

(fn ConstructionScript)